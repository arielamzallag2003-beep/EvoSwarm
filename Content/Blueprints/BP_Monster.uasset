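; Monster actor for an artificial-life simulation that wanders randomly and breeds, spawning with random shape, color, size and stats.
; When its cooldown expires, Tick picks a partner from the GameMode's MonstersList; the nearest-monster check measures self to self, so the last other entry wins.
; TryReproduce spawns a baby at the parents' midpoint, and SetMonster applies averaged traits and either parent's shape.
; Health and Hunger are inherited but otherwise unused.
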(event `self.ReceiveBeginPlay`
  (bind (_returnvalue_location _returnvalue_rotation) (`KismetMathLibrary.BreakTransform` (`self.GetTransform`)))
  (bind _shape (`self.Shape`))
  (bind _shape_2 (`self.Shape`))
  (`|ExecutionSequence`
    (:`then_0`
      (bind _asbp_monster_game_mode (cast `/Game/Blueprints/BP_MonsterGameMode` (`GameplayStatics.GetGameMode`)))
      (set `self.GameMode` _asbp_monster_game_mode))
    (:`then_1`
      (set `self.shapeType` (cast `/Game/Blueprints/E_Shape` (`KismetMathLibrary.Conv_IntToByte` (`KismetMathLibrary.RandomInteger` 4))))
      (set `self.speed` (`KismetMathLibrary.RandomFloatInRange` 0.5 2.0))
      (set `self.health` (`KismetMathLibrary.RandomFloatInRange` 1.0 10.0))
      (set `self.size` (`KismetMathLibrary.RandomFloatInRange` 0.5 2.0))
      (set `self.hunger` (`KismetMathLibrary.RandomFloatInRange` 0.1 1.0))
      (set `self.ReproductionCoolDown` (`KismetMathLibrary.RandomFloatInRange` 1.0 5.0))
      (set `self.color` (`KismetMathLibrary.MakeColor` (`KismetMathLibrary.RandomFloat`) (`KismetMathLibrary.RandomFloat`) (`KismetMathLibrary.RandomFloat`)))
      (switch `/Game/Blueprints/E_Shape` (`self.shapeType`)
        (:`NewEnumerator1`
          (`StaticMeshComponent.SetStaticMesh` _shape "/Engine/BasicShapes/Sphere.Sphere"))
        (:`NewEnumerator2`
          (`StaticMeshComponent.SetStaticMesh` _shape "/Engine/BasicShapes/Cube.Cube"))
        (:`NewEnumerator3`
          (`StaticMeshComponent.SetStaticMesh` _shape "/Engine/BasicShapes/Cone.Cone")))
      (bind _returnvalue (`PrimitiveComponent.CreateDynamicMaterialInstance` _shape_2 0 (`PrimitiveComponent.GetMaterial` _shape_2 0) "None"))
      (`MaterialInstanceDynamic.SetVectorParameterValue` _returnvalue "Color" (`self.color`))
      (`self.K2_SetActorTransform` (`KismetMathLibrary.MakeTransform` _returnvalue_location _returnvalue_rotation (`KismetMathLibrary.Conv_DoubleToVector` (`self.size`)))))))

(event `self.ReceiveTick`
  (params (DeltaSeconds :type "Float (single-precision)"))
  (bind _returnvalue_location (`KismetMathLibrary.BreakTransform` (`self.GetTransform`)))
  (bind _returnvalue_location_2 (`KismetMathLibrary.BreakTransform` (`self.GetTransform`)))
  (bind _nearestmonster (`self.NearestMonster`))
  (bind _reproductioncooldown (`self.ReproductionCoolDown`))
  (bind _returnvalue_location_3 (`KismetMathLibrary.BreakTransform` (`self.GetTransform` (`self.NearestMonster`))))
  (`|ExecutionSequence`
    (:`then_0`
      (if (<= _reproductioncooldown 0.0)
        (set `self.NearestMonster` self)
        (for _array_element (`/Game/Blueprints/BP_MonsterGameMode.MonstersList` (`self.GameMode`))
          (if (!= self _array_element)
            (if (== self _nearestmonster)
              (set `self.NearestMonster` _array_element)
              (elif (<= (`KismetMathLibrary.Vector_Distance` _returnvalue_location _returnvalue_location_2) (`KismetMathLibrary.Vector_Distance` _returnvalue_location _returnvalue_location_3))
                (set `self.NearestMonster` _array_element)))))
        (`self.TryReproduce` _nearestmonster)
        (else
          (set `self.ReproductionCoolDown` (- _reproductioncooldown DeltaSeconds)))))
    (:`then_1`
      (`self.K2_AddActorWorldOffset` (`KismetMathLibrary.MakeVector` (* (`KismetMathLibrary.RandomFloatInRange` -1.0 1.0) (`self.speed`) 5.0) (* (`KismetMathLibrary.RandomFloatInRange` -1.0 1.0) (`self.speed`) 5.0))))))

(fn `SetMonster`
  (params (Monster :type "/Game/Blueprints/BP_Monster Object Reference") (ShapeType :type "/Game/Blueprints/E_Shape Enum" :default "NewEnumerator1") (Speed :type "Float (double-precision)") (Health :type "Float (double-precision)") (Size :type "Float (double-precision)") (Hunger :type "Float (double-precision)") (ReproductionCoolDown :type "Float (double-precision)") (Color :type "LinearColor Structure"))
  (locals (_Monster :type "/Game/Blueprints/BP_Monster Object Reference"))
  (bind _monster (`local.Monster`))
  (bind _monster_2 (`local.Monster`))
  (bind (_returnvalue_location _returnvalue_rotation) (`KismetMathLibrary.BreakTransform` (`self.GetTransform` _monster)))
  (bind _shape (`/Game/Blueprints/BP_Monster.Shape` _monster_2))
  (set `local._Monster` Monster)
  (`|ExecutionSequence`
    (:`then_0`
      (bind _asbp_monster_game_mode (cast `/Game/Blueprints/BP_MonsterGameMode` (`GameplayStatics.GetGameMode`)))
      (set `/Game/Blueprints/BP_Monster.GameMode` _asbp_monster_game_mode (`local.Monster`)))
    (:`then_1`
      (set `/Game/Blueprints/BP_Monster.shapeType` ShapeType _monster))
    (:`then_2`
      (set `/Game/Blueprints/BP_Monster.speed` Speed _monster))
    (:`then_3`
      (set `/Game/Blueprints/BP_Monster.health` Health _monster))
    (:`then_4`
      (set `/Game/Blueprints/BP_Monster.size` Size _monster))
    (:`then_5`
      (set `/Game/Blueprints/BP_Monster.hunger` Hunger _monster))
    (:`then_6`
      (set `/Game/Blueprints/BP_Monster.ReproductionCoolDown` ReproductionCoolDown _monster))
    (:`then_7`
      (set `/Game/Blueprints/BP_Monster.color` Color _monster))
    (:`then_8`
      (switch `/Game/Blueprints/E_Shape` (`/Game/Blueprints/BP_Monster.shapeType` _monster_2)
        (:`NewEnumerator1`
          (`StaticMeshComponent.SetStaticMesh` _shape "/Engine/BasicShapes/Sphere.Sphere"))
        (:`NewEnumerator2`
          (`StaticMeshComponent.SetStaticMesh` _shape "/Engine/BasicShapes/Cube.Cube"))
        (:`NewEnumerator3`
          (`StaticMeshComponent.SetStaticMesh` _shape "/Engine/BasicShapes/Cone.Cone")))
      (bind _returnvalue (`PrimitiveComponent.CreateDynamicMaterialInstance` _shape 0 (`PrimitiveComponent.GetMaterial` _shape 0) "None"))
      (`MaterialInstanceDynamic.SetVectorParameterValue` _returnvalue "Color" (`/Game/Blueprints/BP_Monster.color` (`local.Monster`))))
    (:`then_9`
      (`self.K2_SetActorTransform` _monster (`KismetMathLibrary.MakeTransform` _returnvalue_location _returnvalue_rotation (`KismetMathLibrary.Conv_DoubleToVector` Size)) false false))))

(fn `TryReproduce`
  (params (Parent :type "/Game/Blueprints/BP_Monster Object Reference"))
  (locals (BabyMonster :type "/Game/Blueprints/BP_Monster Object Reference") (BabyShape :type "/Game/Blueprints/E_Shape Enum"))
  (bind _returnvalue_location (`KismetMathLibrary.BreakTransform` (`self.GetTransform` Parent)))
  (bind _returnvalue_location_2 (`KismetMathLibrary.BreakTransform` (`self.GetTransform`)))
  (bind _parent (`local.Parent`))
  (bind (_color_r _color_g _color_b _color_a) (break `LinearColor` (`self.color`)))
  (bind (_color_r_2 _color_g_2) (break `LinearColor` (`/Game/Blueprints/BP_Monster.color` _parent)))
  (if (<= (`/Game/Blueprints/BP_Monster.ReproductionCoolDown` Parent) 0.0)
    (set `/Game/Blueprints/BP_Monster.ReproductionCoolDown` (`KismetMathLibrary.RandomFloatInRange` 2.0 5.0) Parent)
    (set `self.ReproductionCoolDown` (`KismetMathLibrary.RandomFloatInRange` 2.0 5.0))
    (bind _returnvalue (`|SpawnActorFromClass` "BP_Monster_C" (`KismetMathLibrary.MakeTransform` (/ (+ _returnvalue_location_2 _returnvalue_location) (`KismetMathLibrary.Conv_DoubleToVector` 2.0))) "Undefined" "MultiplyWithRoot" null null))
    (bind _output_get (set `local.BabyMonster` _returnvalue))
    (if (`KismetMathLibrary.RandomBool`)
      (set `local.BabyShape` (`self.shapeType`))
      (else
        (set `local.BabyShape` (`/Game/Blueprints/BP_Monster.shapeType` _parent))))
    (`self.SetMonster` _output_get (`local.BabyShape`) (/ (+ (`/Game/Blueprints/BP_Monster.speed` _parent) (`self.speed`)) 2.0) (/ (+ (`/Game/Blueprints/BP_Monster.health` _parent) (`self.health`)) 2.0) (/ (+ (`/Game/Blueprints/BP_Monster.size` _parent) (`self.size`)) 2.0) (/ (+ (`/Game/Blueprints/BP_Monster.hunger` _parent) (`self.hunger`)) 2.0) 5.0 (make `LinearColor` (/ (+ _color_r_2 _color_r) 2.0) (/ (+ _color_g_2 _color_g) 2.0) (/ (+ _color_b _color_a) 2.0) 1.0))
    (`KismetArrayLibrary.Array_Add` (`/Game/Blueprints/BP_MonsterGameMode.MonstersList` (`self.GameMode`)) (`local.BabyMonster`))))

(fn `UserConstructionScript`)