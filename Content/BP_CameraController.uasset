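; Player controller that drives the camera pawn from Enhanced Input.
; On BeginPlay it adds an input mapping context and caches the possessed player pawn as BP_CameraPawn.
; The IA_MoveX and IA_MoveY actions print a debug string and forward their values to the pawn's MoveCameraX and MoveCameraY functions.
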(event `self.ReceiveBeginPlay`
  (`EnhancedInputSubsystemInterface.AddMappingContext` (pcsubsystem `EnhancedInputLocalPlayerSubsystem` self) null 0 (struct))
  (bind _asbp_camera_pawn (cast `/Game/BP_CameraPawn` (`GameplayStatics.GetPlayerPawn` 0)))
  (set `self.Camera Pawn` _asbp_camera_pawn))

(event `EnhancedInput|/Game/IA_MoveX`
  (params (ActionValue :type "Float (double-precision)") (ElapsedSeconds :type "Float (double-precision)") (TriggeredSeconds :type "Float (double-precision)") (InputAction :type "InputAction Object Reference" :default "/Game/IA_MoveX.IA_MoveX"))
  (:`Triggered`
    (`KismetSystemLibrary.PrintString` "X")
    (`/Game/BP_CameraPawn.MoveCameraX` (`self.Camera Pawn`) ActionValue)))

(event `EnhancedInput|/Game/IA_MoveY`
  (params (ActionValue :type "Float (double-precision)") (ElapsedSeconds :type "Float (double-precision)") (TriggeredSeconds :type "Float (double-precision)") (InputAction :type "InputAction Object Reference" :default "/Game/IA_MoveY.IA_MoveY"))
  (:`Triggered`
    (`KismetSystemLibrary.PrintString` "Y")
    (`/Game/BP_CameraPawn.MoveCameraY` (`self.Camera Pawn`) ActionValue)))

(fn `UserConstructionScript`)