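; BP_CameraPawn is a camera pawn that exposes functions to move and rotate the view.
; The move functions offset the actor along world X, Y and Z by input times Speed, so movement ignores the camera's facing.
; Rotation is split: yaw turns the Scene component and pitch turns the SpringArm, both as local rotations of the raw input.
; Its event graph is empty, so these functions run only when called from elsewhere.
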(event `self.ReceiveBeginPlay`)

(fn `MoveCameraX`
  (params (Input :type "Float (double-precision)"))
  (`self.K2_AddActorWorldOffset` (`KismetMathLibrary.MakeVector` (* Input (`self.Speed`)))))

(fn `MoveCameraY`
  (params (Input :type "Float (double-precision)"))
  (`self.K2_AddActorWorldOffset` (`KismetMathLibrary.MakeVector` 0.0 (* Input (`self.Speed`)))))

(fn `MoveCameraZ`
  (params (Input :type "Float (double-precision)"))
  (`self.K2_AddActorWorldOffset` (`KismetMathLibrary.MakeVector` 0.0 0.0 (* Input (`self.Speed`)))))

(fn `RotateCameraY`
  (params (Input :type "Float (double-precision)"))
  (`SceneComponent.K2_AddLocalRotation` (`self.SpringArm`) (`KismetMathLibrary.MakeRotator` 0.0 Input) false false))

(fn `RotateCameraZ`
  (params (Input :type "Float (double-precision)"))
  (`SceneComponent.K2_AddLocalRotation` (`self.Scene`) (`KismetMathLibrary.MakeRotator` 0.0 0.0 Input) false false))

(fn `UserConstructionScript`)